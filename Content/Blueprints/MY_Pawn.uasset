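; Camera pawn for a 360-degree orbit along a camera rail.
; BeginPlay attaches it to the first CameraRig_Rail found, keeping world transform.
; CameraRailRun plays the Loop360Camera timeline, whose update logic maps degrees to rail position, prints the angle and locks orientation to the rail whether or not a look-at target exists.
; Interpolated look-at rotation and forward debug line logic are present but disconnected.
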(event `self.ReceiveBeginPlay`
  ;[1 1 1] 获取相机轨道，并绑定到相机
  (bind _outactors (`GameplayStatics.GetAllActorsOfClass` "/Script/CinematicCamera.CameraRig_Rail"))
  (if (> (`KismetArrayLibrary.Array_Length` _outactors) 0)
    (bind _output_get (set `self.CameralRail` (`|GetArrayItem` _outactors)))
    (`self.K2_AttachToActor` _output_get "None" "KeepWorld" "KeepWorld" "KeepRelative")))

(event `CameraRailRun`
  (`TimelineComponent.PlayFromStart` (`self.Loop360Camera`)))

(fn `UserConstructionScript`)